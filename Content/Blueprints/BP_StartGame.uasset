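; BP_StartGame is an actor that starts the game when it takes any damage, acting as a shootable or hittable start trigger.
; After a two-second delay, it calls SpawnNode on the first BP_Node found in the level and puts a WB_GameTimer widget on screen.
; It then destroys itself and spawns BP_RestartGame at a hardcoded transform, with that spawn sequenced after the DestroyActor call.
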(event `self.ReceiveAnyDamage`
  (params (Damage :type "Float (single-precision)") (DamageType :type "DamageType Object Reference") (InstigatedBy :type "Controller Object Reference") (DamageCauser :type "Actor Object Reference"))
  (`KismetSystemLibrary.Delay` 2.0)
  (`|ExecutionSequence`
    (:`then_0`
      (bind _outactors (`GameplayStatics.GetAllActorsOfClass` "/Game/Blueprints/BP_Node.BP_Node_C"))
      (`/Game/Blueprints/BP_Node.SpawnNode` (`|GetArrayItem` _outactors)))
    (:`then_1`
      (bind _returnvalue (`|CreateWidget` "/Game/UI/WB_GameTimer.WB_GameTimer_C"))
      (bind _output_get (set `self.TimerRef` _returnvalue))
      (`UserWidget.AddToViewport` _output_get 0))
    (:`then_2`
      (`self.K2_DestroyActor`))
    (:`then_3`
      (`|SpawnActorFromClass` "/Game/Blueprints/BP_RestartGame.BP_RestartGame_C" (`KismetMathLibrary.MakeTransform` (70.0 310.0 80.0) (struct :`Yaw` -130.0)) "Undefined" "MultiplyWithRoot" null null))))

(fn `UserConstructionScript`)